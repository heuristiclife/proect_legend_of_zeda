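; Player character Blueprint that handles basic movement and jumping from input bindings.
; The Vertical and Horizontal axis events share one assignment that writes the Direction vector, and the Jump action calls Jump.
; Tick moves the actor by normalized Direction times Speed and delta time using SetActorLocation without sweep, so movement input and collision checks are bypassed.
; EnableInput and AddMovementInput nodes remain unconnected and never run.
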(event EventBeginPlay
  ;[1 1 1] 컨트롤러
)

(event Collision|EventActorBeginOverlap
  (params (OtherActor :type Actor%20Object%20Reference)))

(event EventTick
  (params (DeltaSeconds :type Float%20%28single-precision%29))
  ;[1 1 1] 이동
  (Transformation|SetActorLocation (+ (* (* (Math|Vector|Normalize (Variables|Default|GetDirection)) (Variables|Default|GetSpeed)) DeltaSeconds) (Transformation|GetActorLocation)) false false))

(event Input|ActionEvents|InputActionJump
  (params (Key :type Key%20Structure :default "None"))
  ;[1 1 1] 이동 : 키 바인딩
  (:Pressed
    (Character|Jump)))

(event Input|AxisEvents|InputAxisVertical
  (params (AxisValue :type Float%20%28single-precision%29))
  ;[1 1 1] 이동 : 키 바인딩
  (Variables|Default|SetDirection (Math|Vector|MakeVector AxisValue (stale Input|AxisEvents|InputAxisHorizontal AxisValue) 0.0)))

(event Input|AxisEvents|InputAxisHorizontal
  (params (AxisValue :type Float%20%28single-precision%29))
  ;[1 1 1] 이동 : 키 바인딩
  (Variables|Default|SetDirection (Math|Vector|MakeVector (stale Input|AxisEvents|InputAxisVertical AxisValue) AxisValue 0.0)))

(fn ConstructionScript)